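; First-person player character for a stealth horror game, with movement, interaction, slot inventory, pause menu and camera night vision.
; Camera traces drive the interact dot, item labels and pickups, with inventory use gated on owning the backpack.
; Timelines emit footstep and breath noise events for AI hearing; sneaking and equipment adjust the sneak level that scales footstep noise.
; Breathing turns heavy near the monster and can be held briefly to silence it.
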(event `self.ReceiveTick`
  (params (DeltaSeconds :type "Float (single-precision)"))
  (bind _collectablewidgetref (`self.CollectableWidgetRef`))
  (bind _interact_dot_widget (`self.Interact Dot Widget`))
  (bind _camera (`self.Camera`))
  (bind _returnvalue (`SceneComponent.K2_GetComponentLocation` _camera))
  (bind _returnvalue_2 (`Widget.IsInViewport` (`self.Interact Dot Widget`)))
  ;[1 1 1] CrossHair_BP
  ;;[1 1 1] Determine breath rate
  (`self.SetBreathRate`)
  (`self.Interact Dot Widget`
    (:`then`
      (bind (_outhit _returnvalue_3) (`KismetSystemLibrary.LineTraceSingle` _returnvalue (+ _returnvalue (* (`SceneComponent.GetForwardVector` _camera) (`self.InteractDistance`))) "TraceTypeQuery1"))
      (if _returnvalue_3
        (bind (_bblockinghit _binitialoverlap _time _distance _location _impactpoint _normal _impactnormal _physmat _hitactor) (`GameplayStatics.BreakHitResult` _outhit))
        (if (`KismetSystemLibrary.DoesImplementInterface` _hitactor "/Game/Interactable/BPI_IInteractable.BPI_IInteractable_C")
          (`|ExecutionSequence`
            (:`then_0`
              (if (not _returnvalue_2)
                ;;[1 1 1] Add or remove the dot
                (`UserWidget.AddToViewport` _interact_dot_widget 0)))
            (:`then_1`
              ;;[1 1 1] Big Mess just to get casting only when hovering over item once and then if hover over another you get it again once.
              (if (`KismetSystemLibrary.DoesImplementInterface` _hitactor "/Game/Interactable/Collectable/BPI_PickUp.BPI_PickUp_C")
                (`/Engine/EditorBlueprintResources/StandardMacros.IsValid` (stale _asbp_collectable)
                  (:`Is Valid`
                    (if (and _returnvalue_2 (== (stale _asbp_collectable) _hitactor)) :!label _label
                      _
                      (else
                        (bind _asbp_collectable (cast `/Game/Interactable/Collectable/BP_Collectable` _hitactor :!label _label_2))
                        (set `self.CollectableWidgetRef` (`/Game/Interactable/Collectable/BP_Collectable.Widget` _asbp_collectable))
                        (goto _label))))
                  (:`Is Not Valid`
                    (goto _label_2)))
                (`UserWidget.AddToViewport` _interact_dot_widget 0)
                (`SceneComponent.SetHiddenInGame` _collectablewidgetref false false))))
          (else
            (if _returnvalue_2 :!label _label_3
              (`Widget.RemoveFromParent` _interact_dot_widget)
              (`/Engine/EditorBlueprintResources/StandardMacros.IsValid` _collectablewidgetref
                (:`Is Valid`
                  (`SceneComponent.SetHiddenInGame` _collectablewidgetref true false))))))
        (else
          (goto _label_3))))
    (:`else`)))

(event `self.ReceiveBeginPlay`
  ;[1 1 1] Set default step sound speed
  (`TimelineComponent.SetPlayRate` (`self.FootstepSoundTimeline`) 3.0)
  ;[1 1 1] Start breathing sound emission
  (`TimelineComponent.Play` (`self.EmitBreathSound`))
  ;[1 1 1] Mapping Context
  (`|ExecutionSequence`
    (:`then_0`
      ;[1 1 1] CrossHair_BP
      ;;[1 1 1] Put dot On and Off the screen
      (bind _returnvalue (`|CreateWidget` "/Game/UI/crosshair/InteractDotWidget.InteractDotWidget_C"))
      (set `self.Interact Dot Widget` _returnvalue))
    (:`then_1`
      (`EnhancedInputSubsystemInterface.AddMappingContext` (pcsubsystem `EnhancedInputLocalPlayerSubsystem` (`GameplayStatics.GetPlayerController` 0)) "/Game/Input/IMC_Default.IMC_Default" 0 (struct))
      ;[1 1 1] Get PusRef
      (bind _returnvalue_2 (`GameplayStatics.GetActorOfClass` "/Game/Monsters/BP_Monster_Smart.BP_Monster_Smart_C"))
      (set `self.MonsterRef` _returnvalue_2)
      ;[1 1 1] Added AlwaysShownWidget (because all other widgets are used  for specific things
      (bind _returnvalue_3 (`|CreateWidget` "/Game/UI/BPW_AlwaysVisibleUI.BPW_AlwaysVisibleUI_C" (`GameplayStatics.GetPlayerController` 0)))
      (bind _output_get (set `self.AlwaysVisibleUIRef` _returnvalue_3))
      (`UserWidget.AddToViewport` _output_get 0)
      (bind _asbp_game_mode (cast `/Game/Blueprint/BP_GameMode` (`GameplayStatics.GetGameMode`)))
      (set `self.GameModeRef` _asbp_game_mode)
      ;[1 1 1] Set Slot1 Selected from start
      (`self.OnStartMakeSelectedSlotHighlighted`)
      (bind _returnvalue_4 (`|CreateWidget` "/Game/UI/BPW_InteractItemName.BPW_InteractItemName_C"))
      (set `self.ItemWidgetRef` _returnvalue_4))))

(event `EnhancedInput|/Game/Input/Action/IA_Move`
  (params (ActionValue :type "Vector2D Structure") (ElapsedSeconds :type "Float (double-precision)") (TriggeredSeconds :type "Float (double-precision)") (InputAction :type "InputAction Object Reference" :default "/Game/Input/Action/IA_Move.IA_Move"))
  (bind _footstepsoundtimeline (`self.FootstepSoundTimeline`))
  ;[1 1 1] Add Mapping Context to steer the player
  (:`Triggered`
    (if (not (`self.IsMoveInputIgnored` self))
      (`|ExecutionSequence`
        (:`then_0`
          (`self.AddMovementInput` (`self.GetActorForwardVector`) ActionValue_X))
        (:`then_1`
          (`self.AddMovementInput` (`self.GetActorRightVector`) ActionValue_Y))
        (:`then_2`
          ;[1 1 1] Footstep timeline trigger
          (`TimelineComponent.Play` _footstepsoundtimeline)))))
  (:`Canceled`
    (`TimelineComponent.Stop` _footstepsoundtimeline :!label _label_4))
  (:`Completed`
    (goto _label_4)))

(event `EnhancedInput|/Game/Input/Action/IA_Look`
  (params (ActionValue :type "Vector2D Structure") (ElapsedSeconds :type "Float (double-precision)") (TriggeredSeconds :type "Float (double-precision)") (InputAction :type "InputAction Object Reference" :default "/Game/Input/Action/IA_Look.IA_Look"))
  (bind _mousesens (`self.MouseSens`))
  ;[1 1 1] Camera Mouse Look
  (:`Triggered`
    (`self.AddControllerYawInput` (* ActionValue_X _mousesens))
    (`self.AddControllerPitchInput` (* ActionValue_Y _mousesens))))

(event `InputAction|Interact`
  (params (Key :type "Key Structure"))
  (bind _camera (`self.Camera`))
  (bind _returnvalue (`SceneComponent.K2_GetComponentLocation` _camera))
  ;[1 1 1] Cast trace from the camera when input
  (:`Pressed`
    (bind _outhit (`KismetSystemLibrary.LineTraceSingle` _returnvalue (+ _returnvalue (* (`KismetMathLibrary.GetForwardVector` (`SceneComponent.K2_GetComponentRotation` _camera)) (`KismetSystemLibrary.MakeLiteralDouble` (`self.InteractDistance`)))) "TraceTypeQuery1"))
    (bind (_bblockinghit _binitialoverlap _time _distance _location _impactpoint _normal _impactnormal _physmat _hitactor) (`GameplayStatics.BreakHitResult` _outhit))
    (bind _returnvalue_2 (`KismetSystemLibrary.DoesImplementInterface` _hitactor "/Game/Interactable/BPI_IInteractable.BPI_IInteractable_C"))
    ;[1 1 1] Check if actor is interactable
    (if _returnvalue_2
      (message `/Game/Interactable/BPI_IInteractable.Interact` _hitactor)
      ;[1 1 1] If it Implements interactable and pickup interfaces it casts it to BP_Collectable and adds it to inventory
      (if (and _returnvalue_2 (`KismetSystemLibrary.DoesImplementInterface` _hitactor "/Game/Interactable/Collectable/BPI_PickUp.BPI_PickUp_C") (`/Game/Blueprint/BP_GameMode.HasBackpack` (`self.GameModeRef`)))
        (bind _asbp_collectable (cast `/Game/Interactable/Collectable/BP_Collectable` _hitactor))
        (`/Game/Inventory/BPC_inventory.Add Item To Inventory` (`self.BPC_inventory`) _asbp_collectable)))))

(event `Key|Escape`
  (params (Key :type "Key Structure"))
  (bind _returnvalue (`GameplayStatics.GetPlayerController` 0))
  (bind _pause_menu_ref (`self.Pause Menu Ref`))
  ;[1 1 1] Pause Menu on When M or Esc is pushed
  (:`Pressed`
    (`/Engine/EditorBlueprintResources/StandardMacros.IsValid` (`self.Pause Menu Ref`) :!label _label_5
      (:`Is Valid`
        _)
      (:`Is Not Valid`
        (bind _returnvalue_2 (`|CreateWidget` "/Game/UI/BPW_PauseMenu.BPW_PauseMenu_C"))
        (set `self.Pause Menu Ref` _returnvalue_2)))
    (set `PlayerController.bShowMouseCursor` true _returnvalue)
    (`WidgetBlueprintLibrary.SetInputMode_UIOnlyEx` _returnvalue _pause_menu_ref)
    (`UserWidget.AddToViewport` _pause_menu_ref 0)
    (`GameplayStatics.SetGamePaused` true)))

(event `Key|M`
  (params (Key :type "Key Structure"))
  ;[1 1 1] Pause Menu on When M or Esc is pushed
  (:`Pressed`
    (goto _label_5)))

(event `Add to sneakLevel`
  (params (SneakLevel :type "Float (double-precision)"))
  ;[1 1 1] Set sneakLevel from other classes
  (`self.AddToSneakLevel` SneakLevel))

(event `Key|LeftControl`
  (params (Key :type "Key Structure"))
  ;[1 1 1] Pressing Ctrl makes player halfSpeed(sneaking) and increases sneakLevel
  (:`Pressed`
    (set `self.IsSneaking` true)
    (`self.Sneaking` (`self.IsSneaking`) :!label _label_6))
  (:`Released`
    (set `self.IsSneaking` false)
    (goto _label_6)))

(event `Disable Movement Input`
  (params (StopInput :type Boolean))
  (bind _returnvalue (`GameplayStatics.GetPlayerController` 0))
  ;[1 1 1] Called by BP_Hide when interacting with hide objects disables the movement  only.
  (if StopInput
    (`Controller.SetIgnoreMoveInput` _returnvalue true)
    (else
      (`Controller.ResetIgnoreMoveInput` _returnvalue))))

(event `OnStartMakeSelectedSlotHighlighted`
  (bind _bpc_inventory (`self.BPC_inventory`))
  ;[1 1 1] Convert Key 1-2-3-4 into int and forward that to Selected slot UI
  (`/Game/UI/BPW_InventoryUI.SelectedSlot` (`/Game/Inventory/BPC_inventory.UIRef` _bpc_inventory) (`self.SlotSelected`) :!label _label_7)
  (`/Game/Inventory/BPC_inventory.Display Item Name` _bpc_inventory))

(event `Key|One`
  (params (Key :type "Key Structure"))
  ;[1 1 1] Convert Key 1-2-3-4 into int and forward that to Selected slot UI
  (:`Pressed`
    (`self.KeyToInt` Key)
    (goto _label_7)))

(event `Key|X`
  (params (Key :type "Key Structure"))
  (bind _bpc_inventory (`self.BPC_inventory`))
  (bind _slotselected (`self.SlotSelected`))
  (bind _element (`/Game/Inventory/BPC_inventory.GetElement` _bpc_inventory _slotselected))
  ;[1 1 1] X drops item and removes from inventory, have to check if backPack is picked up else errors
  (:`Pressed`
    (if (`/Game/Blueprint/BP_GameMode.HasBackpack` (`self.GameModeRef`))
      (if (`KismetSystemLibrary.IsValidClass` _element)
        (`/Game/Inventory/BPC_inventory.Drop Item` _bpc_inventory _element)
        (`/Game/Inventory/BPC_inventory.RemoveItemFromInventory` _bpc_inventory _slotselected)
        (`GameplayStatics.PlaySoundAtLocation` "/Game/Inventory/Sounds/DropItem.DropItem" (`self.K2_GetActorLocation`) (struct) 1.0 1.0 0.0 null null null null)))))

(event `Key|Two`
  (params (Key :type "Key Structure"))
  ;[1 1 1] Convert Key 1-2-3-4 into int and forward that to Selected slot UI
  (:`Pressed`
    (`self.KeyToInt` Key)
    (goto _label_7)))

(event `Key|Three`
  (params (Key :type "Key Structure"))
  ;[1 1 1] Convert Key 1-2-3-4 into int and forward that to Selected slot UI
  (:`Pressed`
    (`self.KeyToInt` Key)
    (goto _label_7)))

(event `Key|T`
  (params (Key :type "Key Structure"))
  ;[1 1 1] Temp to test all functionality in inventory array
  (:`Pressed`
    (`/Game/Inventory/BPC_inventory.Print out Inventory` (`self.BPC_inventory`))))

(event `Key|Four`
  (params (Key :type "Key Structure"))
  ;[1 1 1] Convert Key 1-2-3-4 into int and forward that to Selected slot UI
  (:`Pressed`
    (`self.KeyToInt` Key)
    (goto _label_7)))

(event `Key|LeftMouseButton`
  (params (Key :type "Key Structure"))
  (bind _bpc_inventory (`self.BPC_inventory`))
  (bind (_output_itemclass _output_itemicon _output_itemdescription _output_activeactorspawn _output_equipable _output_sneaklevel) (break `/Game/Inventory/InventorySlotStruct` (`|GetArrayItem` (`/Game/Inventory/BPC_inventory.inventory` (`self.BPC_inventory`)) (`self.SlotSelected`))))
  ;[1 1 1] Use Item (aka spawn the Active Item for the Collectable one) if its equipable it calls equip item instead
  (:`Pressed`
    (if (`/Game/Blueprint/BP_GameMode.HasBackpack` (`self.GameModeRef`))
      (if (`KismetSystemLibrary.IsValidClass` _output_itemclass)
        (if _output_equipable
          (`/Game/Inventory/BPC_inventory.EquipItem` _bpc_inventory _output_sneaklevel (`self.SlotSelected`))
          (`GameplayStatics.PlaySoundAtLocation` "/Game/Inventory/Sounds/Equip.Equip" (`self.K2_GetActorLocation`) (struct) 1.0 1.0 0.0 null null null null)
          (else
            (`/Game/Inventory/BPC_inventory.Drop Item` _bpc_inventory _output_activeactorspawn)
            (`/Game/Inventory/BPC_inventory.RemoveItemFromInventory` (`self.BPC_inventory`) (`self.SlotSelected`))
            (`GameplayStatics.PlaySoundAtLocation` "/Game/Inventory/Sounds/DropItem.DropItem" (`self.K2_GetActorLocation`) (struct) 1.0 1.0 0.0 null null null null)))))))

(event `InputAction|ToggleNightvision`
  (params (Key :type "Key Structure"))
  (bind _postprocess (`self.PostProcess`))
  ;[1 1 1] Toggle Night Vision
  (:`Pressed`
    (bind _asbp_game_mode (cast `/Game/Blueprint/BP_GameMode` (`GameplayStatics.GetGameMode`)))
    (if (`/Game/Blueprint/BP_GameMode.HasCamera` _asbp_game_mode)
      (`/Engine/EditorBlueprintResources/StandardMacros.FlipFlop`
        (:`A`
          (bind _returnvalue (`|CreateWidget` "/Game/UI/NightVision/BPW_CameraHUD.BPW_CameraHUD_C" (`GameplayStatics.GetPlayerController` 0)))
          (set `/Game/Blueprint/BP_GameMode.CameraHUD` _returnvalue _asbp_game_mode)
          (`UserWidget.AddToViewport` _returnvalue 0)
          (`Widget.SetVisibility` _returnvalue "Visible")
          (set `PostProcessComponent.bEnabled` true _postprocess))
        (:`B`
          (`Widget.SetVisibility` _returnvalue "Hidden")
          (set `PostProcessComponent.bEnabled` false _postprocess))))))

(event `SetBreathRate`
  (bind _heavybreathing (`self.HeavyBreathing`))
  (bind _regularbreathing (`self.RegularBreathing`))
  ;[1 0.08854 0.08854] Change breath rate logic (on tick)
  (if (< (`self.GetDistanceTo` (`self.MonsterRef`) self) 500.0)
    (if (`AudioComponent.IsPlaying` _regularbreathing)
      (`AudioComponent.Stop` _regularbreathing)
      (`AudioComponent.Play` _heavybreathing 0.0))
    (elif (`AudioComponent.IsPlaying` _heavybreathing)
      (`AudioComponent.Play` _regularbreathing 0.0)
      (`AudioComponent.Stop` _heavybreathing))))

(event `InputAction|HoldBreath`
  (params (Key :type "Key Structure"))
  (bind _emitbreathsound (`self.EmitBreathSound`))
  (bind _regularbreathing (`self.RegularBreathing`))
  ;[1 0 0.6611] Hold Breath / just dont fkin touch it, it was a nightmare to wrap my head around
  (:`Pressed`
    (set `self.KeyIsPressed` true)
    (`TimelineComponent.Stop` _emitbreathsound)
    (`AudioComponent.Stop` _regularbreathing)
    (`AudioComponent.Stop` (`self.HeavyBreathing`))
    (`GameplayStatics.PlaySound2D` "/Game/Blueprint/Sounds/Breathing/Inhale.Inhale" 1.0 1.0 0.0 null null false)
    (`KismetSystemLibrary.Delay` 10.0)
    (if (`self.KeyIsPressed`)
      (set `self.KeyIsPressed` false)
      (`GameplayStatics.PlaySound2D` "/Game/Blueprint/Sounds/Breathing/Exhale.Exhale" 1.0 1.0 0.0 null null false :!label _label)
      (`TimelineComponent.PlayFromStart` _emitbreathsound)
      (`AudioComponent.Play` _regularbreathing 0.0)))
  (:`Released`
    (if (`self.KeyIsPressed`)
      (set `self.KeyIsPressed` false)
      (goto _label))))

(fn `AddToSneakLevel`
  (params (SneakLevel :type "Float (double-precision)"))
  ;[1 1 1] Adds to stealth and is clamped with 1 as max, 0 min
  (set `self.SneakLevel` (`KismetMathLibrary.FClamp` (+ SneakLevel (`self.SneakLevel`)))))

(fn `KeyToInt`
  (params (Key :type "Key Structure" :default "None"))
  ;[1 1 1] Decrease by 1 to match array
  (bind _result (`/Engine/EditorBlueprintResources/StandardMacros.DecrementInt` (`KismetStringLibrary.Conv_StringToInt` (`KismetTextLibrary.Conv_TextToString` (`KismetInputLibrary.Key_GetDisplayName` Key))))
    (:`  `
      (bind _output_get (set `self.SlotSelected` _result))
      (`KismetSystemLibrary.PrintString` (`KismetStringLibrary.Conv_IntToString` _output_get)))))

(fn `Sneaking`
  (params (Condition :type Boolean))
  (locals (SneakSpeedModifier :type "Float (double-precision)" :default 0.5) (DefaultWalkSpeed :type "Float (double-precision)" :default 600.0) (SneakLevelEffect :type "Float (double-precision)" :default 0.3) (DefaultTimelinePlayRate :type "Float (double-precision)" :default 3.0))
  (bind _footstepsoundtimeline (`self.FootstepSoundTimeline`))
  (bind _charactermovement (`self.CharacterMovement`))
  (bind _defaultwalkspeed (`local.DefaultWalkSpeed`))
  (bind _sneakleveleffect (`local.SneakLevelEffect`))
  (bind _defaulttimelineplayrate (`local.DefaultTimelinePlayRate`))
  ;[1 1 1] Comment
  (if Condition
    (set `CharacterMovementComponent.MaxWalkSpeed` (* _defaultwalkspeed (`local.SneakSpeedModifier`)) _charactermovement)
    (`self.AddToSneakLevel` _sneakleveleffect)
    (`TimelineComponent.SetPlayRate` _footstepsoundtimeline (* _defaulttimelineplayrate (`local.SneakSpeedModifier`)))
    (else
      (set `CharacterMovementComponent.MaxWalkSpeed` _defaultwalkspeed _charactermovement)
      (`self.AddToSneakLevel` (* _sneakleveleffect -1.0))
      (`TimelineComponent.SetPlayRate` _footstepsoundtimeline _defaulttimelineplayrate))))

(fn `UserConstructionScript`)