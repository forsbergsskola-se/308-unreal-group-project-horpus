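; Inventory component that manages a four-slot item inventory, mirrored to the game mode's UI and saved in the game instance.
; On BeginPlay it restores the saved inventory and rebuilds the UI list.
; Adding fills the first empty slot, skipping backpack and camera items; adds and removals update both UI and saved copy.
; Helpers show the selected item's description, spawn dropped items before the player and apply equipment sneak bonuses.
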(event `self.ReceiveBeginPlay`
  (bind _asbp_game_mode (cast `/Game/Blueprint/BP_GameMode` (`GameplayStatics.GetGameMode`)))
  (set `self.UIRef` (`/Game/Blueprint/BP_GameMode.UIRef` _asbp_game_mode))
  ;[1 1 1] Set inventory to Saved and loop through to add again to the UI
  (bind _asbp_game_instance (cast `/Game/Blueprint/BP_GameInstance` (`GameplayStatics.GetGameInstance`)))
  (bind _output_get (set `self.GameInstanceRef` _asbp_game_instance))
  (bind (_saved_inventory _inv_size) (`/Game/Blueprint/BP_GameInstance.Set Inventory` _output_get))
  (bind _output_get_2 (set `self.inventory` _saved_inventory))
  (set `self.InvCurrSize` _inv_size)
  (for (_array_element _array_index) _output_get_2
    (`/Game/UI/BPW_InventoryUI.Add Item To List UI` (`self.UIRef`) (`.ItemIcon_9_5C8BA64240BF7C0C142E659EC9DC22FB` (break `/Game/Inventory/InventorySlotStruct` _array_element)) _array_index)))

(fn `Add Item To Inventory`
  (params (NewItem :type "/Game/Interactable/Collectable/BP_Collectable Object Reference (by ref)"))
  (bind _inventoryindex (`self.InventoryIndex`))
  (bind _collectableref (`self.collectableRef`))
  (bind _collectableref_2 (`self.collectableRef`))
  (bind _icon (`self.Get Icon` _collectableref_2))
  (bind _output_get (set `self.collectableRef` NewItem))
  (`KismetSystemLibrary.PrintString` (`KismetSystemLibrary.GetDisplayName` _output_get))
  (cast `/Game/Interactable/Collectable/BP_Backpack` _collectableref
    (:`CastFailed`
      (cast `/Game/Interactable/Collectable/BP_CameraItem` _collectableref
        (:`CastFailed`
          (set `self.InventoryIndex` (`self.CheckFirstEmpty`))
          (bind _output_get_2 (set `self.isInventoryFull` (< (`self.InvCurrSize`) 4)))
          (if _output_get_2
            (`/Game/UI/BPW_InventoryUI.Add Item To List UI` (`self.UIRef`) _icon _inventoryindex)
            (`KismetArrayLibrary.Array_Set` (`self.inventory`) _inventoryindex (make `/Game/Inventory/InventorySlotStruct` (`GameplayStatics.GetObjectClass` _collectableref_2) _icon (`/Game/Interactable/Collectable/BP_Collectable.Item Name` _collectableref_2) (`/Game/Interactable/Collectable/BP_Collectable.ActiveActorToBeSpawned` _collectableref_2) (`/Game/Interactable/Collectable/BP_Collectable.IsEquippable` _collectableref_2) (`/Game/Interactable/Collectable/BP_Collectable.SneakLevel` _collectableref_2)))
            (bind _result (`/Engine/EditorBlueprintResources/StandardMacros.IncrementInt` (`self.InvCurrSize`))
              (:`  `
                (bind _output_get_3 (set `self.InvCurrSize` _result))
                (`/Game/Blueprint/BP_GameInstance.Update Inventory` (`self.GameInstanceRef`) (`self.inventory`) _output_get_3)))
            (else
              (`KismetSystemLibrary.PrintString` "INVENTORY FULL" true true (struct :`R` 1.0 :`B` 0.089516 :`A` 1.0)))))))))

(fn `CheckFirstEmpty`
  (returns (EmptyIndex :type Integer))
  (for (_array_element _array_index) (`self.inventory`)
    (if (not (`KismetSystemLibrary.IsValidClass` (break `/Game/Inventory/InventorySlotStruct` _array_element)))
      (return _array_index))))

(fn `Display Item Name`
  (bind _asbp_player (cast `/Game/Blueprint/BP_Player` (`GameplayStatics.GetPlayerCharacter` 0)))
  (bind (_output_itemclass _output_itemicon _output_itemdescription) (break `/Game/Inventory/InventorySlotStruct` (`|GetArrayItem` (`self.inventory`) (`/Game/Blueprint/BP_Player.SlotSelected` _asbp_player))))
  (`/Game/UI/BPW_InventoryUI.Display Item Text` (`self.UIRef`) _output_itemdescription))

(fn `Drop Item`
  (params (Actor :type "Actor Class Reference"))
  (bind _returnvalue (`GameplayStatics.GetPlayerCharacter` 0))
  (bind (_returnvalue_location _returnvalue_rotation _returnvalue_scale) (`KismetMathLibrary.BreakTransform` (`Actor.GetTransform` _returnvalue)))
  ;[1 1 1] Spawn selected Item infront of player
  (`|SpawnActorFromClass` Actor (`KismetMathLibrary.MakeTransform` (+ _returnvalue_location (* (`SceneComponent.GetForwardVector` (`Character.Mesh` _returnvalue)) 150)) _returnvalue_rotation _returnvalue_scale) "Undefined" "MultiplyWithRoot" null null)
  (return))

(fn `EquipItem`
  (params (SneakIncrease :type "Float (double-precision)"))
  (bind _asbp_player (cast `/Game/Blueprint/BP_Player` (`GameplayStatics.GetPlayerCharacter` 0)))
  (`/Game/Blueprint/BP_Player.Add to sneakLevel` _asbp_player SneakIncrease))

(fn `Get Icon`
  (params (collectableRef :type "/Game/Interactable/Collectable/BP_Collectable Object Reference"))
  (returns (Icon :type "Texture2D Object Reference"))
  (return (`/Game/Interactable/Collectable/BP_Collectable.Icon` collectableRef)))

(fn `GetElement`
  (params (index :type Integer))
  (returns (element :type "/Game/Interactable/Collectable/BP_Collectable Class Reference"))
  (bind _output_itemclass (break `/Game/Inventory/InventorySlotStruct` (`|GetArrayItem` (`self.inventory`) index)))
  (return _output_itemclass))

(fn `Print out Inventory`
  (for _array_element (`self.inventory`)
    (`KismetSystemLibrary.PrintString` (`KismetSystemLibrary.GetClassDisplayName` (break `/Game/Inventory/InventorySlotStruct` _array_element)))))

(fn `RemoveItemFromInventory`
  (params (SelectedSlot :type Integer))
  (`/Game/UI/BPW_InventoryUI.Remove Item From UI List` (`self.UIRef`) SelectedSlot)
  (`KismetArrayLibrary.Array_Set` (`self.inventory`) SelectedSlot)
  (bind _result (`/Engine/EditorBlueprintResources/StandardMacros.DecrementInt` (`self.InvCurrSize`))
    (:`  `
      (bind _output_get (set `self.InvCurrSize` _result))
      (`/Game/Blueprint/BP_GameInstance.Update Inventory` (`self.GameInstanceRef`) (`self.inventory`) _output_get))))