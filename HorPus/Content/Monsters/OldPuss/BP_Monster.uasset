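; BP_Monster is a monster character that records its spawn transform on BeginPlay and can be toggled to haunt the player.
; ToggleHaunt sets walk speed and alternates via FlipFlop between AI-moving to the player and returning to spawn, restoring its original rotation on arrival.
; GetTrapped zeroes walk speed for the effect's duration, then restores it; TrapStrength is unused.
; SetPlayerStealth only stores the player's stealth level.
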(event `self.ReceiveBeginPlay`
  (bind (_returnvalue_location _returnvalue_rotation) (`KismetMathLibrary.BreakTransform` (`self.GetTransform`)))
  ;[1 1 1] Set variables
  (set `self.SpawnPoint` _returnvalue_location)
  (set `self.SpawnRotation` _returnvalue_rotation))

(event `ToggleHaunt`
  ;[1 1 1] Move to player
  (set `CharacterMovementComponent.MaxWalkSpeed` 600.0 (`self.CharacterMovement`))
  (`/Engine/EditorBlueprintResources/StandardMacros.FlipFlop`
    (:`A`
      (`|AIMoveTo` self (0.0 0.0 0.0) (`GameplayStatics.GetPlayerCharacter` 0)))
    (:`B`
      ;[1 1 1] Go back to spawner
      (`|AIMoveTo` self (`self.SpawnPoint`) null
        (:`OnSuccess`
          (`self.K2_SetActorRotation` (`self.SpawnRotation`)))))))

(event `SetPlayerStealth`
  (params (NewStealthLevel :type "Float (double-precision)"))
  ;[1 1 1] Set Player Stealth
  (set `self.PlayerStealthLevel` NewStealthLevel))

(event `GetTrapped`
  (params (TrapStrength :type "Float (double-precision)") (EffectiveTime :type "Float (double-precision)"))
  (bind _charactermovement (`self.CharacterMovement`))
  ;[1 1 1] GetTrapped
  (bind _output_get (set `self.OriginalWalkSpeed` (`CharacterMovementComponent.MaxWalkSpeed` _charactermovement)))
  (set `CharacterMovementComponent.MaxWalkSpeed` 0.0 _charactermovement)
  (`KismetSystemLibrary.Delay` EffectiveTime)
  (set `CharacterMovementComponent.MaxWalkSpeed` _output_get _charactermovement))

(fn `UserConstructionScript`)