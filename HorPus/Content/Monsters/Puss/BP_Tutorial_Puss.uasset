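; Tutorial cat monster (Puss) that meows until the player interacts with it, ending the tutorial in a staged death.
; A timeline started on BeginPlay drives random meow sounds at the cat's location.
; Interact advances the game mode's mission once, freezes the cat with emissive eyes and stops the meowing.
; It then disables player input and movement, plays an angry sound, shows the death screen and loads MainLevel after a short delay.
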(event `self.ReceiveBeginPlay`
  (`TimelineComponent.Play` (`self.MeowingTimeLine`)))

(event `/Game/Interactable/BPI_Interactable.Interact`
  (bind _returnvalue (`GameplayStatics.GetPlayerCharacter` 0))
  (`|ExecutionSequence`
    (:`then_0`
      (`/Engine/EditorBlueprintResources/StandardMacros.DoOnce` false
        (:`Completed`
          (bind _asbp_game_mode (cast `/Game/Blueprint/BP_GameMode` (`GameplayStatics.GetGameMode`)))
          (bind _asbp_player (cast `/Game/Blueprint/BP_Player` (`GameplayStatics.GetPlayerPawn` 0)))
          (`/Game/Blueprint/BP_GameMode.Get Next Mission` _asbp_game_mode (`/Game/Blueprint/BP_Player.AlwaysVisibleUIRef` _asbp_player)))))
    (:`then_1`
      (`PrimitiveComponent.SetMaterial` (`self.SkeletalMesh`) 0 "/Game/Monsters/Puss/Assets/MuchkinEmmisiveEyes.MuchkinEmmisiveEyes")
      (`SkeletalMeshComponent.Stop` (`self.SkeletalMesh`))
      (`self.DisableInput` _returnvalue (`GameplayStatics.GetPlayerController` 0))
      (bind _asbp_player_2 (cast `/Game/Blueprint/BP_Player` _returnvalue))
      (`TimelineComponent.Stop` (`self.MeowingTimeLine`))
      (`GameplayStatics.PlaySoundAtLocation` "/Game/Monsters/Puss/Assets/Sounds/angry_kitty.angry_kitty" (`self.K2_GetActorLocation`) (struct) 1.0 1.0 0.0 "/Game/Monsters/Tasks/NewSoundAttenuation.NewSoundAttenuation" "/Game/Monsters/Tasks/NewSoundConcurrency.NewSoundConcurrency" null null)
      (`CharacterMovementComponent.DisableMovement` (`Character.CharacterMovement` _asbp_player_2))
      (bind _returnvalue_2 (`|CreateWidget` "/Game/UI/BPW_DeathScreen.BPW_DeathScreen_C"))
      (`UserWidget.AddToViewport` _returnvalue_2 0)
      (`KismetSystemLibrary.Delay` 1.5)
      (`GameplayStatics.OpenLevel` "MainLevel"))))

(fn `UserConstructionScript`)