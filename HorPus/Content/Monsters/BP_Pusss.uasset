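; BP_Pusss is a monster pawn that chases the player while haunting and otherwise returns to its starting spot.
; The construction script records its location as the spawn point.
; The IsHaunting event checks a haunting flag and runs AI MoveTo toward either the player character or that spawn point.
; On successfully reaching the spawn point, it snaps its rotation once to face the player.
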(event `IsHaunting`
  (bind _returnvalue (`self.K2_GetActorLocation`))
  ;[1 1 1] Move to player
  (if (`self.isHaunted_0`)
    (`|AIMoveTo` self (0.0 0.0 0.0) (`GameplayStatics.GetPlayerCharacter` 0))
    (else
      (`|AIMoveTo` self (`self.SpawnPoint_0`) null
        (:`OnSuccess`
          ;[1 1 1] Look at player
          (`self.K2_SetActorLocationAndRotation` _returnvalue (`KismetMathLibrary.FindLookAtRotation` _returnvalue (`self.K2_GetActorLocation` (`GameplayStatics.GetPlayerCharacter` 0)))))))))

(fn `UserConstructionScript`
  (set `self.SpawnPoint_0` (`self.K2_GetActorLocation`)))