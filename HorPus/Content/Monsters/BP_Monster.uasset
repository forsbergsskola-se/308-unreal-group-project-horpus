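; BP_Monster is a monster pawn that alternates between haunting the player and returning to its spawn point.
; On BeginPlay it caches its starting location and rotation.
; Each ToggleHaunt call flips between AI moving toward the player character and moving back to the cached spawn point.
; After a successful return it restores its original facing.
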(event `self.ReceiveBeginPlay`
  (bind (_returnvalue_location _returnvalue_rotation) (`KismetMathLibrary.BreakTransform` (`self.GetTransform`)))
  ;[1 1 1] Set variables
  (set `self.SpawnPoint` _returnvalue_location)
  (set `self.SpawnRotation` _returnvalue_rotation))

(event `ToggleHaunt`
  ;[1 1 1] Move to player
  (`/Engine/EditorBlueprintResources/StandardMacros.FlipFlop`
    (:`A`
      (`|AIMoveTo` self (0.0 0.0 0.0) (`GameplayStatics.GetPlayerCharacter` 0)))
    (:`B`
      ;[1 1 1] Go back to spawner
      (`|AIMoveTo` self (`self.SpawnPoint`) null
        (:`OnSuccess`
          (`self.K2_SetActorRotation` (`self.SpawnRotation`)))))))

(fn `UserConstructionScript`)