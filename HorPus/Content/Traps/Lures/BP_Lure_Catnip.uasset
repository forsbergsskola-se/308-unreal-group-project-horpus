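; Catnip lure trap that switches the AI monster's sight over to its lured perception when an actor overlaps it.
; BeginPlay sets the trap's strength, while construction and overlap both call the parent's logic first.
; On any overlap, it gets the monster from BP_GameMode, disables sight on its normal perception component and enables sight on the lured one.
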(event `self.ReceiveBeginPlay`
  ;[1 1 1] Set trap strength
  (set `self.Strength` 0.5))

(event `self.ReceiveActorBeginOverlap`
  (params (OtherActor :type "Actor Object Reference"))
  (`parent.ReceiveActorBeginOverlap` OtherActor)
  (bind _asbp_game_mode (cast `/Game/Blueprint/BP_GameMode` (`GameplayStatics.GetGameMode`)))
  (bind _output_get (set `self.AI_Monster` (`/Game/Blueprint/BP_GameMode.MonsterReference` _asbp_game_mode)))
  ;[0.2898 0.9502 1] Change to Lure perception (Sight) BTTask_DestroyLure
  (`AIPerceptionComponent.SetSenseEnabled` (`/Game/Monsters/AI_Monster_Smart.AIPerception` _output_get) "/Script/AIModule.AISense_Sight" false)
  (`AIPerceptionComponent.SetSenseEnabled` (`/Game/Monsters/AI_Monster_Smart.AIPerception_Lured` _output_get) "/Script/AIModule.AISense_Sight" true))

(fn `UserConstructionScript`
  (`parent.UserConstructionScript`))