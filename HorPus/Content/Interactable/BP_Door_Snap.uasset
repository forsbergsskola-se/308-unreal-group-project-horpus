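; Interactable swinging door that the player can open and close when unlocked, and that the monster can open when pathing through it.
; A child-actor NavLinkProxy detects the monster arriving and, if the door is closed and off cooldown, sets OnNavLink and Door on its blackboard.
; MonsterOpenDoor and Interact share a FlipFlop-driven rotation timeline.
; Monster opening blocks player interaction until shortly after the door fully opens.
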(event `self.ReceiveBeginPlay`
  ;[1 1 1] When puss is on navlink
  (bind _asnav_link_proxy (cast `NavLinkProxy` (`ChildActorComponent.ChildActor` (`self.ChildActor`))))
  (add `NavLinkProxy.OnSmartLinkReached` _asnav_link_proxy (delegate `MonsterAtDoor`)))

(event `MonsterAtDoor`
  (params (MovingActor :type "Actor Object Reference") (DestinationPoint :type "Vector Structure (by ref)"))
  (if (not (or (`self.IsOpen`) (`self.IsOnCooldown`)))
    (bind _asbp_monster_smart (cast `/Game/Monsters/BP_Monster_Smart` MovingActor))
    (bind _returnvalue (`AIBlueprintHelperLibrary.GetBlackboard` _asbp_monster_smart))
    ;[0.05805 0.1878 1] Set blackboard variables
    (`BlackboardComponent.SetValueAsBool` _returnvalue "OnNavLink" true)
    (`BlackboardComponent.SetValueAsObject` _returnvalue "Door" self)))

(event `MonsterOpenDoor`
  ;[1 0 0.009271] Prevents the player closing the door while puss is trying to get through
  (set `self.IsOnCooldown` true)
  (`GameplayStatics.PlaySound2D` "/Game/Interactable/SFX/open-and-closed-door.open-and-closed-door" 0.2 1.0 0.0 "/Game/UI/MainMenuCon.MainMenuCon" null :!label _label)
  (`/Engine/EditorBlueprintResources/StandardMacros.FlipFlop`
    (:`A`
      ;[1 1 1] Door animation
      (bind (_direction _doormovement) (`Timeline|MovementTime` :!label _label_2)
        (:`Update`
          (`SceneComponent.K2_SetRelativeRotation` (`self.SM_Door`) (`KismetMathLibrary.MakeRotator` 0.0 0.0 _doormovement) false false)
          (if (== _doormovement -90.0)
            (set `self.IsOpen` true)
            ;[1 1 1] Wait until puss is through the door
            (`KismetSystemLibrary.Delay` 1.0)
            (set `self.IsOnCooldown` false)
            (else
              (set `self.IsOpen` false))))))
    (:`B`
      (goto _label_2 :!via `Reverse`))))

(event `/Game/Interactable/BPI_IInteractable.Interact`
  ;[1 0 0.009271] Prevents the player closing the door while puss is trying to get through
  (if (`self.IsOnCooldown`)
    _
    (elif (`self.IsUnlocked`)
      (goto _label)
      (else
        (`GameplayStatics.PlaySoundAtLocation` "/Game/Interactable/SFX/LockedDoor.LockedDoor" (`self.K2_GetActorLocation`) (struct) 1.0 1.0 0.0 null "/Game/UI/MainMenuCon.MainMenuCon" null null)))))

(fn `UserConstructionScript`)