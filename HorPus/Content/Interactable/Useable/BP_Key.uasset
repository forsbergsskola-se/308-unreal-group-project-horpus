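; BP_Key is a useable key item, labeled for opening doors, that advances the mission when the player interacts with it.
; On Interact it runs the parent logic, then sets its keys icon and item name.
; It then calls GetNextMission on BP_GameMode, passing the player's always-visible UI reference.
; PickUpItem is empty, and the construction script only calls its parent.
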(event `/Game/Interactable/BPI_IInteractable.Interact`
  (`parent.Interact`)
  (set `self.Icon` "/Game/Textures/Keys-Icon.Keys-Icon")
  (set `self.Item Name` "Keys: \nUse to Open Door")
  (bind _asbp_game_mode (cast `/Game/Blueprint/BP_GameMode` (`GameplayStatics.GetGameMode`)))
  (bind _asbp_player (cast `/Game/Blueprint/BP_Player` (`GameplayStatics.GetPlayerCharacter` 0)))
  (`/Game/Blueprint/BP_GameMode.Get Next Mission` _asbp_game_mode (`/Game/Blueprint/BP_Player.AlwaysVisibleUIRef` _asbp_player)))

(fn `Pick Up Item`
  (returns (item :type "/Game/Interactable/Collectable/BP_Collectable Object Reference"))
  (return null))

(fn `UserConstructionScript`
  (`parent.UserConstructionScript`))