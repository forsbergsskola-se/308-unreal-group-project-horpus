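; BP_Backpack is an interactable backpack collectable.
; On BeginPlay it enables an outline on its backpack mesh.
; Interacting calls its Interacted override, which has BP_GameMode show the UI and then runs the parent's interaction logic, skipping both if the game mode cast fails.
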(event `self.ReceiveBeginPlay`
  ;[1 1 1] Enable outline
  (`self.EnableOutline` (`self.large_backpack_-_white_texture_mockup`)))

(event `/Game/Interactable/BPI_IInteractable.Interact`
  ;[1 1 1] Enable interact
  (`self.Interacted`))

(fn `Interacted`
  (bind _asbp_game_mode (cast `/Game/Blueprint/BP_GameMode` (`GameplayStatics.GetGameMode`)))
  (`/Game/Blueprint/BP_GameMode.ShowUI` _asbp_game_mode)
  (`parent.Interacted`))

(fn `UserConstructionScript`
  (`parent.UserConstructionScript`))