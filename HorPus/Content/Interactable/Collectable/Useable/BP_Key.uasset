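; BP_Key is a useable collectable key item that the player can interact with.
; On BeginPlay it calls the parent logic, then sets its item name and icon to Keys, and Interact simply defers to the parent.
; A disconnected collapsed graph, which never runs, would once advance the GameMode to the next mission in the Tinker level using the player's always-visible UI.
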(event `self.ReceiveBeginPlay`
  (`parent.ReceiveBeginPlay`)
  (set `self.Item Name` "Keys")
  (set `self.Icon` "/Game/Textures/Keys-Icon.Keys-Icon"))

(event `/Game/Interactable/BPI_Interactable.Interact`
  (`parent.Interact`))

(fn `UserConstructionScript`
  (`parent.UserConstructionScript`))