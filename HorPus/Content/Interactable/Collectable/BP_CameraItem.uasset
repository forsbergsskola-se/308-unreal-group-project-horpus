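; BP_CameraItem is the collectable camera pickup that the player can interact with once they have a backpack.
; Interacting sets HasCamera on the game mode, saves it to the game instance, lights up the UI camera icon and destroys the actor, or shows a "no backpack" message.
; BeginPlay restores HasCamera from the game instance and re-tints the icon after a short delay to wait for the UI reference.
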(event `self.ReceiveBeginPlay`
  ;[1 1 1] OnStart Check if we already picked up camera to show UI
  (`parent.ReceiveBeginPlay`)
  (bind _asbp_game_instance (cast `/Game/Blueprint/BP_GameInstance` (`GameplayStatics.GetGameInstance`)))
  (bind _savedcamera (`/Game/Blueprint/BP_GameInstance.Get currCamera` _asbp_game_instance))
  (bind _asbp_game_mode (cast `/Game/Blueprint/BP_GameMode` (`GameplayStatics.GetGameMode`)))
  (bind _output_get (set `/Game/Blueprint/BP_GameMode.HasCamera` _savedcamera _asbp_game_mode))
  (if _output_get
    ;[1 1 1] Add delay because of initiation order (needs to wait for UIRef to set
    (`KismetSystemLibrary.Delay` 0.2)
    (`Image.SetBrushTintColor` (`/Game/UI/BPW_InventoryUI.CameraImage` (`/Game/Blueprint/BP_GameMode.UIRef` _asbp_game_mode)) (make `SlateColor` (struct :`R` 1.0 :`G` 1.0 :`B` 1.0 :`A` 1.0)))))

(event `/Game/Interactable/BPI_IInteractable.Interact`
  ;[1 1 1] Enable interact
  (bind _asbp_game_mode (cast `/Game/Blueprint/BP_GameMode` (`GameplayStatics.GetGameMode`)))
  (if (`/Game/Blueprint/BP_GameMode.HasBackpack` _asbp_game_mode)
    (bind _output_get (set `/Game/Blueprint/BP_GameMode.HasCamera` true _asbp_game_mode))
    ;[1 1 1] Set CameraPickedUp save
    (bind _asbp_game_instance (cast `/Game/Blueprint/BP_GameInstance` (`GameplayStatics.GetGameInstance`)))
    (`/Game/Blueprint/BP_GameInstance.SetCamera` _asbp_game_instance _output_get)
    (`Image.SetBrushTintColor` (`/Game/UI/BPW_InventoryUI.CameraImage` (`/Game/Blueprint/BP_GameMode.UIRef` _asbp_game_mode)) (make `SlateColor` (struct :`R` 1.0 :`G` 1.0 :`B` 1.0 :`A` 1.0)))
    (`self.K2_DestroyActor`)
    (else
      (bind _asbp_player (cast `/Game/Blueprint/BP_Player` (`GameplayStatics.GetPlayerCharacter` 0)))
      (`/Game/UI/BPW_AlwaysVisibleUI.Display Text For Always Show UI` (`/Game/Blueprint/BP_Player.AlwaysVisibleUIRef` _asbp_player) "You dont have a backpack!"))))

(fn `UserConstructionScript`
  (`parent.UserConstructionScript`))