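; BP_Collectable is a physics-simulated world collectable that outlines itself when the player is nearby.
; BeginPlay gathers the static meshes under MeshParent and enables physics on them.
; Each Tick, a visibility trace toward the player toggles their custom depth stencil outline when unblocked and within range.
; Interact is an empty stub; the backpack check, full-inventory check and destroy logic are disconnected and never run.
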(event `self.ReceiveBeginPlay`
  (`self.GenerateMeshArray`)
  (for _array_element (`self.MeshArray`)
    (`PrimitiveComponent.SetSimulatePhysics` _array_element true)))

(event `self.ReceiveTick`
  (params (DeltaSeconds :type "Float (single-precision)"))
  (`self.CheckOutline`))

(event `/Game/Interactable/BPI_Interactable.Interact`
  ;[0.0812 1 0] Make add to inventory event
)

(fn `CheckOutline`
  (bind _returnvalue (`GameplayStatics.GetPlayerCharacter` 0))
  (bind _mesharray (`self.MeshArray`))
  (`/Engine/EditorBlueprintResources/StandardMacros.IsValid` _returnvalue
    (:`Is Valid`
      (bind _outhit (`KismetSystemLibrary.LineTraceSingle` (`self.K2_GetActorLocation`) (`self.K2_GetActorLocation` _returnvalue) "TraceTypeQuery1"))
      (if (and (not (`GameplayStatics.BreakHitResult` _outhit)) (< (`KismetMathLibrary.Vector_Distance` (`.TraceStart` (`GameplayStatics.BreakHitResult` _outhit)) (`.TraceEnd` (`GameplayStatics.BreakHitResult` _outhit))) 500.0))
        (for _array_element _mesharray
          (`self.EnableOutline` _array_element))
        (else
          (for _array_element_2 _mesharray
            (`self.DisableOutline` _array_element_2)))))))

(fn `DisableOutline`
  (params (Mesh :type "PrimitiveComponent Object Reference"))
  (`PrimitiveComponent.SetRenderCustomDepth` Mesh false))

(fn `EnableOutline`
  (params (Mesh :type "StaticMeshComponent Object Reference"))
  (`PrimitiveComponent.SetRenderCustomDepth` Mesh true)
  (`PrimitiveComponent.SetCustomDepthStencilValue` Mesh 2))

(fn `GenerateMeshArray`
  (for _array_element (`SceneComponent.GetChildrenComponents` (`self.MeshParent`) false)
    (bind _asstatic_mesh_component (cast `StaticMeshComponent` _array_element))
    (`KismetArrayLibrary.Array_Add` (`self.MeshArray`) _asstatic_mesh_component)))

(fn `UserConstructionScript`)