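; BP_Shoes is an equippable collectable for sneakers, described to the player as raising sneak level when equipped.
; It extends a parent interactable, setting its item name on BeginPlay after the parent's logic runs.
; On Interact, it calls the parent first, then assigns the shoe icon, a descriptive item name and a fixed sneak level.
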(event `self.ReceiveBeginPlay`
  (`parent.ReceiveBeginPlay`)
  (set `self.Item Name` "Sneakers"))

(event `/Game/Interactable/BPI_Interactable.Interact`
  (`parent.Interact`)
  (set `self.Icon` "/Game/StarterContent/Shoes-Icon.Shoes-Icon")
  (set `self.Item Name` "Sneakers: \nEquip to increase sneak level")
  (set `self.SneakLevel` 0.5))

(fn `UserConstructionScript`
  (`parent.UserConstructionScript`))