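; Wardrobe hiding place that extends a parent interactable and animates its two doors when used.
; Interact calls the parent, then, if interaction is enabled or the player is inside, plays a timeline that yaws both doors through OpenClose.
; A DoOnce, reset on each interaction, reverses the timeline once so the doors close automatically after opening.
; Overlap events track IsOverlapping, intended to prevent opening without entering.
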(event `self.ReceiveActorBeginOverlap`
  (params (OtherActor :type "Actor Object Reference"))
  (`parent.ReceiveActorBeginOverlap` OtherActor)
  ;[1 1 1] So we cant open the door without also entering (overlapp and interact)
  (set `self.IsOverlapping` true))

(event `self.ReceiveActorEndOverlap`
  (params (OtherActor :type "Actor Object Reference"))
  (`parent.ReceiveActorEndOverlap` OtherActor)
  ;[1 1 1] So we cant open the door without also entering (overlapp and interact)
  (set `self.IsOverlapping` false))

(event `/Game/Interactable/BPI_IInteractable.Interact`
  (`parent.Interact`)
  (if (or (`self.InteractEnabled`) (not (`self.OutsideOfHidingplace`)))
    (`|ExecutionSequence`
      (:`then_0`
        (bind (_direction _rightdoor _leftdoor) (`Timeline|Open/Close Doors` :!label _label)
          (:`Update`
            (`self.OpenClose` (.z _rightdoor) _leftdoor))
          (:`Finished`
            (`/Engine/EditorBlueprintResources/StandardMacros.DoOnce` false :!label _label_2
              (:`Completed`
                (goto _label :!via `Reverse`))))))
      (:`then_1`
        (goto _label_2 :!via `Reset`)))))

(fn `OpenClose`
  (params (RightDoor :type "Float (double-precision)") (LeftDoor :type "Float (double-precision)"))
  (bind (_relativerotation_roll _relativerotation_pitch) (`KismetMathLibrary.BreakRotator` (`SceneComponent.RelativeRotation` (`self.Wardrobe_LeftDoor`))))
  (bind (_relativerotation_roll_2 _relativerotation_pitch_2) (`KismetMathLibrary.BreakRotator` (`SceneComponent.RelativeRotation` (`self.Wardrobe_RightDoor`))))
  (`|ExecutionSequence`
    (:`then_0`
      (`SceneComponent.K2_SetRelativeRotation` (`self.Wardrobe_RightDoor`) (`KismetMathLibrary.MakeRotator` _relativerotation_roll_2 _relativerotation_pitch_2 (* RightDoor 75.0)) false false))
    (:`then_1`
      (`SceneComponent.K2_SetRelativeRotation` (`self.Wardrobe_LeftDoor`) (`KismetMathLibrary.MakeRotator` _relativerotation_roll _relativerotation_pitch (+ (* LeftDoor 75.0) 100.0)) false false))))

(fn `UserConstructionScript`
  (`parent.UserConstructionScript`))