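; Interactable hiding spot that moves the player into and back out of a hiding box, usable while the player overlaps it.
; Interact flip-flops a Timeline between play and reverse, lerping player XY from the saved start position to the box.
; The start position is saved only when animation progress is zero, so mid-animation toggles keep it.
; Both CalcAnimationHeight branches scale player Z toward world zero, not box height.
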(event `self.ReceiveActorBeginOverlap`
  (params (OtherActor :type "Actor Object Reference"))
  ;[1 1 1] Enable/disable interact based on player begin/end overlap
  (if (== OtherActor (`GameplayStatics.GetPlayerCharacter` 0))
    (set `self.InteractEnabled` true)))

(event `self.ReceiveBeginPlay`
  ;[1 1 1] Set variable on BeginPlay
  (set `self.HidingPlaceLocation` (`SceneComponent.K2_GetComponentLocation` (`self.HidingPlaceBox`))))

(event `self.ReceiveActorEndOverlap`
  (params (OtherActor :type "Actor Object Reference"))
  ;[1 1 1] Enable/disable interact based on player begin/end overlap
  (if (== (`GameplayStatics.GetPlayerCharacter` 0) OtherActor)
    (set `self.InteractEnabled` false)))

(event `/Game/Interactable/BPI_IInteractable.Interact`
  (bind (_originalplayerlocation_x _originalplayerlocation_y _originalplayerlocation_z) (`KismetMathLibrary.BreakVector` (`self.OriginalPlayerLocation`)))
  (bind (_hidingplacelocation_x _hidingplacelocation_y) (`KismetMathLibrary.BreakVector` (`self.HidingPlaceLocation`)))
  (bind (_returnvalue_x _returnvalue_y _returnvalue_z) (`KismetMathLibrary.BreakVector` (`SceneComponent.K2_GetComponentLocation` (`self.HidingPlaceBox`))))
  ;[1 1 1] Hide
  ;;[1 1 1] if (interactEnabled)
  (if (`self.InteractEnabled`)
    ;;[1 1 1] Set PlayerCharacterInfo variable
    (set `self.PlayerCharacterInfo` (`GameplayStatics.GetPlayerCharacter` 0))
    (`/Engine/EditorBlueprintResources/StandardMacros.FlipFlop`
      (:`A`
        ;;[1 1 1] If actor is not mid-animation
        (if (== 0.0 (`self.AnimationProgress`))
          ;;;[1 1 1] Update OriginaPlayerLocation variable
          (set `self.OriginalPlayerLocation` (`self.K2_GetActorLocation` (`self.PlayerCharacterInfo`)))
          ;;[1 1 1] Character animation timeline
          (bind (_direction _movealpha _heightalpha _progress) (`Timeline|Timeline` :!label _label)
            (:`Update`
              (bind _newheight (`self.calcAnimationHeight` _heightalpha _originalplayerlocation_z _returnvalue_z))
              (set `self.AnimationProgress` _progress)
              (bind (_returnvalue_x_2 _returnvalue_y_2) (`KismetMathLibrary.BreakVector` (`KismetMathLibrary.VLerp` (`KismetMathLibrary.MakeVector` _originalplayerlocation_x _originalplayerlocation_y _originalplayerlocation_z) (`KismetMathLibrary.MakeVector` _hidingplacelocation_x _hidingplacelocation_y) _movealpha)))
              (`self.K2_SetActorLocation` (`self.PlayerCharacterInfo`) (`KismetMathLibrary.MakeVector` _returnvalue_x_2 _returnvalue_y_2 _newheight) false false)))
          (else
            (goto _label))))
      (:`B`
        (goto _label :!via `Reverse`)))))

(fn `calcAnimationHeight`
  (params (Alpha :type "Float (double-precision)") (PlayerZ :type "Float (double-precision)") (HideBoxZ :type "Float (double-precision)"))
  (returns (newHeight :type "Float (double-precision)"))
  (bind _output_get (set `self.IsPlayerBiggerThanBox` (>= PlayerZ HideBoxZ)))
  (if _output_get
    (return (- PlayerZ (* PlayerZ Alpha)))
    (else
      (return (* (- 1.0 Alpha) PlayerZ)))))

(fn `UserConstructionScript`)